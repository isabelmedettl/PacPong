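; BP_Pac is a self-moving ball pawn that starts on a random diagonal and bounces off walls and paddles.
; Wall hits reflect its velocity, while paddle hits steer it by impact point and normal and reset the multiplier, both debounced by DoOnce with short delays.
; Overlapping pickups raises multiplier and score.
; Enemies deal damage unless it is Powered, stopping it and triggering death at zero health.
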(event OnComponentBeginOverlap(SphereComponent)
  (params (OverlappedComponent :type Primitive%20Component%20Object%20Reference) (OtherActor :type Actor%20Object%20Reference) (OtherComp :type Primitive%20Component%20Object%20Reference) (OtherBodyIndex :type Integer) (bFromSweep :type Boolean) (SweepResult :type Hit%20Result%20Structure%20%28by%20ref%29))
  (bind _aspick_up (Utilities|Casting|CastToPickUp OtherActor)
    (:then
      (Class|PickUp|PickUpFunc _aspick_up)
      (bind _output_get (Variables|Default|SetMultiplier (+ (Variables|Default|GetMultiplier) 1)))
      (Variables|Default|SetScore (+ (Variables|Default|GetScore) (* _output_get (Variables|/Script/PacPong.PickUp|GetScoreValue _aspick_up))))
      (Audio|PlaySound2D "/Game/Audio/SFX/PickupCue.PickupCue" 1.0 1.0 0.0 0 0))
    (:CastFailed
      (bind _asbp_enemy (Utilities|Casting|CastToBP_Enemy OtherActor))
      (if (not (Variables|Default|GetbPowered))
        (Variables|Default|SetCurrentHealth (- (Variables|Default|GetCurrentHealth) (Variables|/Script/PacPong.Enemy|GetDamage _asbp_enemy)))
        (if (<= (Variables|Default|GetCurrentHealth) 0)
          (Variables|Default|SetVelocity "0, 0, 0")
          (Variables|/Script/Engine.FloatingPawnMovement|SetMaxSpeed (Variables|Default|GetMovementComponent) 0.0)
          (Class|Pac|DoDeath))))))

(event OnComponentHit(MeshComponent)
  (params (HitComponent :type Primitive%20Component%20Object%20Reference) (OtherActor :type Actor%20Object%20Reference) (OtherComp :type Primitive%20Component%20Object%20Reference) (NormalImpulse :type Vector :default "0, 0, 0") (Hit :type Hit%20Result%20Structure%20%28by%20ref%29))
  (bind (_bblockinghit _binitialoverlap _time _distance _location _impactpoint _normal _impactnormal _physmat _hitactor _hitcomponent) (Collision|BreakHitResult Hit))
  (Utilities|Casting|CastToBP_Walls OtherActor
    (:then
      (Utilities|FlowControl|DoOnce false :!label _label
        (:Completed
          (Variables|Default|SetVelocity (Math|Vector|GetReflectionVector (Variables|Default|GetVelocity) _impactnormal))
          (Audio|PlaySound2D "/Game/Audio/SFX/WallBounceCue.WallBounceCue" 1.0 1.0 0.0 0 0)
          (Utilities|FlowControl|Delay 0.1)
          (goto _label Reset))))
    (:CastFailed
      (Utilities|Casting|CastToBP_Paddle OtherActor)
      (Utilities|FlowControl|DoOnce false :!label _label_2
        (:Completed
          (Variables|Default|SetVelocity (* (Math|Vector|Normalize (+ (Math|Vector|Normalize (- _impactpoint (Transformation|GetWorldLocation _hitcomponent))) _impactnormal)) (Math|Vector|VectorLength (Variables|Default|GetVelocity))))
          (Variables|Default|SetMultiplier 0)
          (Audio|PlaySound2D "/Game/Audio/SFX/JumpCue.JumpCue" 1.0 1.0 0.0 0 0)
          (Utilities|FlowControl|Delay 0.1)
          (goto _label_2 Reset))))))

(event EventBeginPlay
  (Variables|Default|SetVelocity (Math|Vector|MakeVector (Math|Conversions|ToFloat(Integer) (Math|Integer|SelectInt 1 -1 (Math|Random|RandomBool))) (Math|Conversions|ToFloat(Integer) (Math|Integer|SelectInt 1 -1 (Math|Random|RandomBool))) 0.0)))

(event EventTick
  (params (DeltaSeconds :type Float%20%28single-precision%29))
  (Class|PawnMovementComponent|AddInputVector (Variables|Default|GetMovementComponent) (Variables|Default|GetVelocity) false))

(fn ConstructionScript)