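; BP_PickUpManager escalates the Pac-Pong music each time its ResetEvent fires.
; Each reset plays an arcade win jingle and increments AmountOfResets, normally nudging the theme's pitch up by 0.1.
; When the count hits three, a DoOnce instead sets the theme's sound to the Ver 2 track and drops its pitch to a slower base, from which later resets climb again.
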(event EventBeginPlay)

(event Collision|EventActorBeginOverlap
  (params (OtherActor :type Actor%20Object%20Reference)))

(event EventTick
  (params (DeltaSeconds :type Float%20%28single-precision%29)))

(event EventResetEvent
  (bind _pac_pong_theme_0605_ver_2 (Variables|Default|GetPAC_PONG_THEME_0605_Ver_2))
  (bind _pac_pong_theme_0605_ver_2_2 (Variables|Default|GetPAC_PONG_THEME_0605_Ver_2))
  (Audio|PlaySound2D "/Game/Audio/SFX/ESM_Melodic_Win_1_Arcade_80s_Simple_Alert_Notification_Game.ESM_Melodic_Win_1_Arcade_80s_Simple_Alert_Notification_Game" 1.0 1.0 0.0 0 0)
  (bind _result (Math|Integer|IncrementInt (Variables|Default|GetAmountOfResets))
    (:%20%20
      (if (== _result 3)
        (Utilities|FlowControl|DoOnce false
          (:Completed
            (Audio|Components|Audio|SetSound _pac_pong_theme_0605_ver_2_2 "/Game/Audio/PAC_PONG_THEME_0605_Ver_2.PAC_PONG_THEME_0605_Ver_2")
            (Audio|Components|Audio|SetPitchMultiplier _pac_pong_theme_0605_ver_2_2 0.8)))
        (else
          (Audio|Components|Audio|SetPitchMultiplier _pac_pong_theme_0605_ver_2 (+ (Variables|/Script/Engine.AudioComponent|GetPitchMultiplier _pac_pong_theme_0605_ver_2) 0.1)))))))

(fn ConstructionScript)