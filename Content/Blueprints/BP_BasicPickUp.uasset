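; BP_BasicPickUp is a basic pickup that reports its collection to a Manager.
; Its PickUpFunc event decrements the Manager's count of basic pickups left, disables mesh collision and toggles mesh visibility instead of destroying the actor.
; When the count reaches zero, it calls ResetPickUps on the Manager.
; The event has no trigger in this Blueprint, and the construction script is empty.
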(event EventBeginPlay)

(event Collision|EventActorBeginOverlap
  (params (OtherActor :type Actor%20Object%20Reference)))

(event EventTick
  (params (DeltaSeconds :type Float%20%28single-precision%29)))

(event EventPickUpFunc
  (bind _manager (Variables|Default|GetManager))
  (bind _output_get (Variables|/Script/PacPong.PickUpManager|SetNumberOfBasicPickUpsLeft _manager (- (Variables|/Script/PacPong.PickUpManager|GetNumberOfBasicPickUpsLeft _manager) 1)))
  (Collision|SetCollisionProfileName (Variables|Default|GetMeshComponent) "NoCollision" true :!class /Script/Engine.PrimitiveComponent)
  (Rendering|ToggleVisibility (Variables|Default|GetMeshComponent) false)
  (if (== _output_get 0)
    (Class|PickUpManager|ResetPickUps _manager)))

(fn ConstructionScript)