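; Paddle controller Blueprint that toggles the game's pause menu from the Enhanced Input pause action.
; Pausing creates and stores a UWBP_PauseMenu widget, adds it to the viewport, sets Game and UI input focused on it, and pauses the game.
; Unpausing removes the widget, resumes the game and restores game-only input.
; The IsPauseMenuOpened flag selects the branch, and both branches set the mouse cursor visible.
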(event Input|EnhancedActionEvents|EnhancedInputActionIA_PauseGame
  (params (ActionValue :type Boolean) (ElapsedSeconds :type Float%20%28double-precision%29) (TriggeredSeconds :type Float%20%28double-precision%29) (InputAction :type Input%20Action%20Object%20Reference :default "/Game/IA_PauseGame.IA_PauseGame"))
  (bind _returnvalue (Game|GetPlayerController 0))
  (:Started
    (if (not (Variables|Default|GetisPauseMenuOpened))
      ;[1 1 1] Pause
      (Variables|Default|SetisPauseMenuOpened true)
      (bind _returnvalue_2 (UserInterface|CreateWidget "/Game/Assets/UI/UWBP_PauseMenu.UWBP_PauseMenu_C" _returnvalue))
      (bind _output_get (Variables|Default|SetPause%20Menu%20Widget _returnvalue_2))
      (UserInterface|Viewport|AddtoViewport _output_get 0)
      (Input|SetInputModeGameandUI _returnvalue (Variables|Default|GetPause%20Menu%20Widget) "DoNotLock" true false)
      (Variables|/Script/Engine.PlayerController|SetbShowMouseCursor _returnvalue true)
      (Game|SetGamePaused true)
      (else
        ;[1 1 1] Unpause
        (Variables|Default|SetisPauseMenuOpened false)
        (Widget|RemovefromParent (Variables|Default|GetPause%20Menu%20Widget))
        (Game|SetGamePaused false)
        (Input|SetInputModeGameOnly _returnvalue false)
        (Variables|/Script/Engine.PlayerController|SetbShowMouseCursor _returnvalue true)))))

(event EventBeginPlay)

(event EventTick
  (params (DeltaSeconds :type Float%20%28single-precision%29)))

(fn ConstructionScript)